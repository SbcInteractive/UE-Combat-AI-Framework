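; Enemy character with a health component, an overhead health bar and a melee attack against the player.
; BeginPlay links the health component to the bar widget, which Tick keeps turned toward the camera.
; DoAttack plays a montage whose notifies open and close the hit window.
; During that window, Tick sphere-traces the left hand's path between frames, applying damage once per swing, reduced if the player blocks.
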(event `self.ReceiveBeginPlay`
  (bind _ac_health (`self.AC_Health`))
  ; Inicializar la barra de vida
  (bind _aswbp_enemy_health_bar (cast `/Game/UI/Enemy/WBP_EnemyHealthBar` (`WidgetComponent.GetWidget` (`self.Widget`))))
  (set `/Game/UI/Enemy/WBP_EnemyHealthBar.EnemyHealth` _ac_health _aswbp_enemy_health_bar)
  (`/Game/AC_Health.OnHealthChanged` _ac_health (`/Game/AC_Health.CurrentHealth` _ac_health) (`/Game/AC_Health.MaxHealth` _ac_health) false))

(event `self.ReceiveTick`
  (params (DeltaSeconds :type "Float (single-precision)"))
  (bind _returnvalue (`SceneComponent.GetSocketLocation` (`self.Mesh`) "LeftHandSocket"))
  (`|ExecutionSequence`
    (:`then_0`
      ; Actualiza cosas constantes, como hacer que la barra de vida mire siempre hacia la cámara del jugador
      (`SceneComponent.K2_SetWorldRotation` (`self.Widget`) (`KismetMathLibrary.FindLookAtRotation` (`SceneComponent.K2_GetComponentLocation` (`self.Widget`)) (`PlayerCameraManager.GetCameraLocation` (`GameplayStatics.GetPlayerCameraManager` 0))) false false))
    (:`then_1`
      (if (`self.IsAttack?`)
        ; Hace el trazado de la espada, confirma si golpeó al jugador y le aplica el daño
        (bind (_outhit _returnvalue_2) (`KismetSystemLibrary.SphereTraceSingleForObjects` :`Start` (`self.ManoAnterior`) :`End` _returnvalue :`Radius` 20.0 :`ObjectTypes` (`|MakeArray` "ObjectTypeQuery3" :!type "EObjectTypeQuery Enum") :`DrawDebugType` "ForDuration" :`DrawTime` 1.0))
        (set `self.ManoAnterior` _returnvalue)
        (if _returnvalue_2
          (bind _asbp_third_person_character (cast `/Game/ThirdPerson/Blueprints/BP_ThirdPersonCharacter` (`.HitActor` (`GameplayStatics.BreakHitResult` _outhit))))
          (`/Engine/EditorBlueprintResources/StandardMacros.DoOnce` false :!label _label
            (:`Completed`
              (if (`/Game/ThirdPerson/Blueprints/BP_ThirdPersonCharacter.bEstaBloqueando` _asbp_third_person_character)
                (bind _returnvalue_3 (`self.GetComponentByClass` _asbp_third_person_character "/Game/AC_Health.AC_Health_C"))
                (`/Game/AC_Health.TakeDamage` _returnvalue_3 5.0)
                (else
                  (`/Game/AC_Health.TakeDamage` _returnvalue_3 20.0))))))))))

(event `ResetearFiltroDeDaño`
  ; Hace el trazado de la espada, confirma si golpeó al jugador y le aplica el daño
  (goto _label :!via `Reset`))

(event `DoAttack`
  ; Ejecuta la animación y la lógica para que el enemigo golpee al jugador
  (bind _notifyname (`|PlayMontage` (`self.Mesh`) "/Game/EnemyCharacter/Animations/Attack_Montage.Attack_Montage")
    (:`OnNotifyBegin`
      (switch `name` _notifyname
        (:`IniciarAtaque`
          (`|ExecutionSequence`
            (:`then_0`
              (set `self.ManoAnterior` (`SceneComponent.GetSocketLocation` (`self.Mesh`) "LeftHandSocket"))
              (set `self.IsAttack?` true))
            (:`then_1`
              (`self.ResetearFiltroDeDaño`))))
        (:`FinAtaque`
          (set `self.IsAttack?` false))))))

(fn `NewFunction`)

(fn `UserConstructionScript`)