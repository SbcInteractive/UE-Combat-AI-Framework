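; Health component that tracks an owner's current and maximum health.
; BeginPlay fills current health to the maximum, then redundantly writes that value back to the maximum.
; TakeDamage subtracts damage with clamping, prints the result, and broadcasts OnHealthChanged with current and maximum values.
; It also broadcasts OnDeath whenever health is zero after a hit, with no guard against repeat calls.
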(event `self.ReceiveBeginPlay`
  (bind _output_get (set `self.CurrentHealth` (`self.MaxHealth`)))
  (set `self.MaxHealth` _output_get))

(fn `TakeDamage`
  (params (DamageAmount :type "Float (double-precision)"))
  (bind _output_get (set `self.CurrentHealth` (`KismetMathLibrary.FClamp` (- (`self.CurrentHealth`) DamageAmount) 0.0 (`self.MaxHealth`))))
  (`KismetSystemLibrary.PrintString` (`KismetStringLibrary.Conv_DoubleToString` _output_get))
  (`self.OnHealthChanged` _output_get (`self.MaxHealth`))
  (if (<= _output_get 0.0)
    (`self.OnDeath`)))